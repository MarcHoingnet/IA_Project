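; AI controller for BP_NPC that runs BT_NPC and supplies patrol destinations from the pawn's NavPoints.
; On BeginPlay it caches the pawn, starts the tree and writes the next nav point location to the NextDestination blackboard key.
; GetNextDestination advances an index that wraps around the array by modulo.
; Perception updates only print actors whose first tag matches TagTarget; SetTargetDestination is an empty stub.
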(event OnTargetPerceptionUpdated(AIPerception)
  (params (Actor :type Actor%20Object%20Reference) (Stimulus :type AI%20Stimulus%20Structure))
  (if (== (Utilities|Array|Get(acopy) (Variables|/Script/Engine.Actor|GetTags Actor)) (Variables|Default|GetTagTarget))
    (Development|PrintString (Utilities|GetObjectName Actor))))

(event EventBeginPlay
  (bind _asbp_npc (Utilities|Casting|CastToBP_NPC (Pawn|GetControlledPawn)))
  (Variables|Default|SetAs%20BP%20NPC _asbp_npc)
  (AI|RunBehaviorTree "/Game/Blueprint/BT_NPC.BT_NPC")
  (bind _destination (CallFunction|GetNextDestination))
  (CallFunction|SetNextDestination _destination))

(fn ConstructionScript)

(fn GetNextDestination
  (bind _as_bp_npc (Variables|Default|GetAs%20BP%20NPC))
  (bind _navpoints (Variables|/Game/Blueprint/BP_NPC.BP_NPC_C|GetNavPoints _as_bp_npc))
  (bind _output_get (Variables|Default|SetActualNavPointsIndex (+ (Variables|Default|GetActualNavPointsIndex) 1)))
  (return (Transformation|GetActorLocation (Utilities|Array|Get(acopy) _navpoints (Math|Integer|%(Integer) _output_get (Utilities|Array|Length _navpoints))))))

(fn SetTargetDestination)

(fn SetNextDestination
  (params (Destination :type Vector))
  (AI|Components|Blackboard|SetValueasVector (Variables|Default|GetBlackboard) (Utilities|Name|MakeLiteralName "NextDestination") Destination))